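; BP_BuildingManager manages building placement previews, spawning a BP_BuildingMaster for a requested row name.
; SetPreview calls DestoryPreview if a preview is active, then spawns the new building and sets the previewing flag.
; The spawn location snaps the externally set cursor position's X and Y to a grid, then the building receives a construction status.
; DestoryPreview is an empty stub, and nothing here moves the preview after spawning.
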(event Custom|SetPreview
  (params (RowName :type Name))
  (if (Preview|GetIsPreviewing)
    (CallFunction|DestoryPreview))
  (CallFunction|SpawnPreviewBuilding RowName)
  (Preview|SetIsPreviewing true))

(event Custom|SpawnPreviewBuilding
  (params (RowName :type Name))
  (Variables|Preview|SetPreviewTransform (Math|Conversions|ToTransform(Vector) (CallFunction|GetGridSnaps)))
  (bind _returnvalue (Game|SpawnActorfromClass "/Game/Building/Buildings/BP_BuildingMaster.BP_BuildingMaster_C" (Variables|Preview|GetPreviewTransform) "AdjustIfPossibleButAlwaysSpawn" "MultiplyWithRoot" 0 RowName "NewEnumerator0" 0))
  (Utilities|IsValid _returnvalue
    (:Is%20Valid
      (bind _output_get (Variables|References|SetBuildingRef _returnvalue))
      (Default|SetConstructionStatus _output_get "NewEnumerator0"))))

(event Custom|Destory%20Preview)

(event EventBeginPlay)

(event EventTick
  (params (DeltaSeconds :type Float%20%28single-precision%29)))

(fn GetIsPreviewing
  (return (Variables|Preview|GetbisPreviewing)))

(fn SetIsPreviewing
  (params (bisPreviewing :type Boolean))
  (Variables|Preview|SetbisPreviewing bisPreviewing)
  (return))

(fn GetGridSnaps
  (bind _cursor_position (Variables|Preview|GetCursor%20Position))
  (bind _snapvalues (Variables|References|GetSnapValues))
  (bind _snapvalues_2 (Variables|References|GetSnapValues))
  (return (Math|Vector|MakeVector (Math|Conversions|ToFloat(Integer) (* (/ (Math|Float|Floor (+ (.x _cursor_position) 5e+01)) _snapvalues) _snapvalues)) (Math|Conversions|ToFloat(Integer) (* (/ (Math|Float|Floor (+ (.y _cursor_position) 5e+01)) _snapvalues_2) _snapvalues_2)) (.z _cursor_position))))

(fn SetCursorPosition
  (params (CursorPosition :type Vector))
  (Variables|Preview|SetCursor%20Position CursorPosition)
  (return))